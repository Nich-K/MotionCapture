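; A two-sided door Blueprint that opens and closes both leaves when the player presses E nearby.
; A box trigger enables input from player controller 0 on overlap and disables it on exit.
; Each E press flips two FlipFlops that play or reverse separate timelines, which set the yaw of the left and right door meshes.
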(event OnComponentBeginOverlap(BoxTrigger)
  (params (OverlappedComponent :type Primitive%20Component%20Object%20Reference) (OtherActor :type Actor%20Object%20Reference) (OtherComp :type Primitive%20Component%20Object%20Reference) (OtherBodyIndex :type Integer) (bFromSweep :type Boolean) (SweepResult :type Hit%20Result%20Structure%20%28by%20ref%29))
  (Input|EnableInput (Game|GetPlayerController 0)))

(event OnComponentEndOverlap(BoxTrigger)
  (params (OverlappedComponent :type Primitive%20Component%20Object%20Reference) (OtherActor :type Actor%20Object%20Reference) (OtherComp :type Primitive%20Component%20Object%20Reference) (OtherBodyIndex :type Integer))
  (Input|DisableInput (Game|GetPlayerController 0)))

(event Input|KeyboardEvents|E
  (params (Key :type Key%20Structure :default "None"))
  (:Pressed
    (Utilities|FlowControl|FlipFlop
      (:A
        (bind _dooropen (Timeline|Timeline_1 Play)
          (:Update
            (Transformation|SetRelativeRotation (Variables|Default|GetDoor_2sided_L) (Math|Rotator|MakeRotator 0.0 0.0 _dooropen) false false))))
      (:B
        (Timeline|Timeline_1 Reverse)))))

(event Input|KeyboardEvents|E
  (params (Key :type Key%20Structure :default "None"))
  (:Pressed
    (Utilities|FlowControl|FlipFlop
      (:A
        (bind _dooropen (Timeline|Timeline_0 Play)
          (:Update
            (Transformation|SetRelativeRotation (Variables|Default|GetDoor_2sided_R) (Math|Rotator|MakeRotator 0.0 0.0 _dooropen) false false))))
      (:B
        (Timeline|Timeline_0 Reverse)))))

(fn ConstructionScript)